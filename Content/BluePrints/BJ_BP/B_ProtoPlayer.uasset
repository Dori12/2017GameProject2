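; B_ProtoPlayer is a prototype player character with camera-relative movement, look, jump and item pickup.
; Axis inputs move along control yaw and turn the controller, with rate-scaled variants and optional pitch inversion.
; LookUP also rotates the Camera's pitch directly, ignoring the invert setting.
; Overlapping a B_ProtoItem tagged "Item" stores it in GetItem, which is never cleared on leaving, and the Active action destroys it.
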(event Custom|ItemGet
  ;[1 1 1] 아이템 획득 관련
  (Actor|DestroyActor (Variables|Default|GetGetItem)))

(event Collision|EventActorBeginOverlap
  (params (OtherActor :type Actor%20Object%20Reference))
  ;[1 1 1] 아이템 획득 관련
  (if (Actor|ActorHasTag OtherActor "Item")
    (bind _asb_proto_item (Utilities|Casting|CastToB_ProtoItem OtherActor))
    (Variables|Default|SetGetItem _asb_proto_item)))

(event Input|ActionEvents|InputActionJump
  (params (Key :type Key%20Structure :default "AnyKey"))
  ;[1 1 1] 이동 및 카메라 조작
  (:Pressed
    (Character|Jump)))

(event Input|ActionEvents|InputActionActive
  (params (Key :type Key%20Structure :default "AnyKey"))
  ;[1 1 1] 아이템 획득 관련
  (:Pressed
    (if (Utilities|IsValid (Variables|Default|GetGetItem))
      (CallFunction|ItemGet))))

(event Input|AxisEvents|InputAxisMoveForward
  (params (AxisValue :type Float%20%28single-precision%29))
  ;[1 1 1] 이동 및 카메라 조작
  (Pawn|Input|AddMovementInput (Math|Vector|GetForwardVector (Math|Rotator|MakeRotator 0.0 0.0 (.Yaw (Math|Rotator|BreakRotator (Pawn|GetControlRotation :!class /Script/Engine.Pawn))))) AxisValue false))

(event Input|AxisEvents|InputAxisLookUP
  (params (AxisValue :type Float%20%28single-precision%29))
  (bind _returnvalue (* AxisValue -1.0))
  ;[1 1 1] 이동 및 카메라 조작
  (if (Variables|조작|GetInvertMouseControl)
    (Pawn|Input|AddControllerPitchInput _returnvalue)
    (else
      (Pawn|Input|AddControllerPitchInput AxisValue)))
  (Transformation|AddRelativeRotation (Variables|Default|GetCamera) (Math|Rotator|MakeRotator 0.0 _returnvalue 0.0) false false))

(event Input|AxisEvents|InputAxisMoveRight
  (params (AxisValue :type Float%20%28single-precision%29))
  ;[1 1 1] 이동 및 카메라 조작
  (Pawn|Input|AddMovementInput (Math|Vector|GetRightVector (Math|Rotator|MakeRotator 0.0 0.0 (.Yaw (Math|Rotator|BreakRotator (Pawn|GetControlRotation :!class /Script/Engine.Pawn))))) AxisValue false))

(event Input|AxisEvents|InputAxisTurn
  (params (AxisValue :type Float%20%28single-precision%29))
  ;[1 1 1] 이동 및 카메라 조작
  (Pawn|Input|AddControllerYawInput AxisValue))

(event Input|AxisEvents|InputAxisTurnRate
  (params (AxisValue :type Float%20%28single-precision%29))
  ;[1 1 1] 이동 및 카메라 조작
  (Pawn|Input|AddControllerYawInput (* AxisValue (Variables|조작|GetBaseTurnRate) (Utilities|Time|GetWorldDeltaSeconds))))

(event Input|AxisEvents|InputAxisLookUpRate
  (params (AxisValue :type Float%20%28single-precision%29))
  ;[1 1 1] 이동 및 카메라 조작
  (Pawn|Input|AddControllerPitchInput (* AxisValue (Variables|조작|GetBaseLookUpRate) (Utilities|Time|GetWorldDeltaSeconds))))

(fn ConstructionScript)